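; BP_Board is the chess board actor that registers its squares and key pieces with the game mode.
; On BeginPlay it casts the game mode to GM_Chess and copies its Squares, Engine, both kings and all four rooks into it.
; It holds no other logic; the construction script and other events are empty.
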(event `self.ReceiveBeginPlay`
  ;[1 1 1] Gives game mode references to squares on start
  (bind _asgm_chess (cast `/Game/Chess/Blueprints/GM_Chess` (`GameplayStatics.GetGameMode`)))
  (set `/Game/Chess/Blueprints/GM_Chess.Squares` (`self.Squares`) _asgm_chess)
  (set `/Game/Chess/Blueprints/GM_Chess.Engine` (`self.Engine`) _asgm_chess)
  (set `/Game/Chess/Blueprints/GM_Chess.WhiteKing` (`self.WhiteKing`) _asgm_chess)
  (set `/Game/Chess/Blueprints/GM_Chess.BlackKing` (`self.BlackKing`) _asgm_chess)
  (set `/Game/Chess/Blueprints/GM_Chess.WhiteRookQ` (`self.WhiteRookQ`) _asgm_chess)
  (set `/Game/Chess/Blueprints/GM_Chess.WhiteRookK` (`self.WhiteRookK`) _asgm_chess)
  (set `/Game/Chess/Blueprints/GM_Chess.BlackRookQ` (`self.BlackRookQ`) _asgm_chess)
  (set `/Game/Chess/Blueprints/GM_Chess.BlackRookK` (`self.BlackRookK`) _asgm_chess))

(fn `UserConstructionScript`)