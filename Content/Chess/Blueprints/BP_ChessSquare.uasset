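; BP_ChessSquare is a single chess board square that changes its mesh material to show highlight states.
; On BeginPlay it caches the mesh's first material as the default.
; Its functions swap that material slot to a highlight or capture-highlight material instance, or restore the cached default.
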(event `self.ReceiveBeginPlay`
  (set `self.DefaultMaterial` (`PrimitiveComponent.GetMaterial` (`self.MeshComp`) 0)))

(fn `SetDefault`
  (`PrimitiveComponent.SetMaterial` (`self.MeshComp`) 0 (`self.DefaultMaterial`)))

(fn `SetHighlighted`
  (`PrimitiveComponent.SetMaterial` (`self.MeshComp`) 0 "/Game/Chess/Materials/MI_BoardHighlighted.MI_BoardHighlighted"))

(fn `SetHighlightedCapture`
  (`PrimitiveComponent.SetMaterial` (`self.MeshComp`) 0 "/Game/Chess/Materials/MI_BoardHighlightedCapture.MI_BoardHighlightedCapture"))

(fn `UserConstructionScript`)