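; Chess engine actor that talks to a UCI-style engine and plays its moves for Black on the board.
; A state machine gates the exchange: wait for "uciok", send a FEN position, request a timed search, then parse "bestmove".
; Move coordinates map to GM_Chess squares, and a timeline moves the piece in an arc with physics off.
; On finish it re-enables physics, reports the move to GM_Chess and awaits the next position.
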(event `self.OnOutput`
  (params (Message :type String))
  (bind (_fromx _fromy _tox _toy) (`self.StringToCoord` (`KismetStringLibrary.GetSubstring` Message 9 4)))
  (switch `EChessEngineState` (`self.EngineState`)
    (:`E_STARTING`
      ;[1 1 1] Waiting for "uciok"
      (if (== (`KismetStringLibrary.GetSubstring` Message 0 5) "uciok")
        (set `self.EngineState` "E_WAITING_FOR_POSITION")
        (`KismetSystemLibrary.PrintString` "Ready")))
    (:`E_WAITING_FOR_POSITION`)
    (:`E_CALCULATING_MOVE`
      (if (== (`KismetStringLibrary.GetSubstring` Message 0 8) "bestmove")
        (`KismetSystemLibrary.PrintString` "move found")
        (bind _asgm_chess (cast `/Game/Chess/Blueprints/GM_Chess` (`GameplayStatics.GetGameMode`)))
        (bind _squares (`/Game/Chess/Blueprints/GM_Chess.Squares` _asgm_chess))
        (bind _output (`|GetArrayItem` _squares (`/Game/Chess/Blueprints/GM_Chess.To1d` _asgm_chess _fromx _fromy)))
        (bind _currentpawn (`/Game/Chess/Blueprints/BP_ChessSquare.CurrentPawn` _output))
        (if (`KismetSystemLibrary.IsValid` _currentpawn)
          (bind _output_get (set `self.PawnToMove` _currentpawn))
          (`/Game/Chess/Blueprints/BP_ChessPawn.SetSimluatePhysics` _output_get false)
          (bind (_direction _z _horizontal) (`Timeline|MovePawn` :!via `PlayFromStart`)
            (:`Update`
              (bind _output_2 (`|GetArrayItem` _squares (`/Game/Chess/Blueprints/GM_Chess.To1d` _asgm_chess _tox _toy)))
              (`self.K2_SetActorLocation` _output_get (`KismetMathLibrary.MakeVector` (`KismetMathLibrary.FInterpTo` (.x (`self.K2_GetActorLocation` _output)) (.x (`self.K2_GetActorLocation` _output_2)) _horizontal 1.0) (`KismetMathLibrary.FInterpTo` (.y (`self.K2_GetActorLocation` _output)) (.y (`self.K2_GetActorLocation` _output_2)) _horizontal 1.0) (+ (.z (`self.K2_GetActorLocation` _output)) (* _z 75.0))) false false))
            (:`Finished`
              (`/Game/Chess/Blueprints/BP_ChessPawn.SetSimluatePhysics` _output_get true)
              (bind _asgm_chess_2 (cast `/Game/Chess/Blueprints/GM_Chess` (`GameplayStatics.GetGameMode`)))
              (`/Game/Chess/Blueprints/GM_Chess.PerformMove` _asgm_chess_2 "E_Black" _output_2 _output_get)
              (`/Game/Chess/Blueprints/GM_Chess.ResetHighlights` _asgm_chess_2 false)
              (set `self.EngineState` "E_WAITING_FOR_POSITION")))
          (else
            (`KismetSystemLibrary.PrintString` (`KismetStringLibrary.Concat_StrStr` "no valid pawn at: " (`KismetStringLibrary.Conv_IntToString` _fromx) ";" (`KismetStringLibrary.Conv_IntToString` _fromy)))))))))

(event `self.ReceiveBeginPlay`
  (`KismetSystemLibrary.Delay` 2.0)
  (`self.StartEngine`))

(event `self.ReceiveTick`
  (params (DeltaSeconds :type "Float (single-precision)")))

(fn `StartCalculateMove`
  (if (`|EnumEquality` (`self.EngineState`) "E_WAITING_FOR_COMMAND")
    (set `self.EngineState` "E_CALCULATING_MOVE")
    (`self.SendCommand` (`KismetStringLibrary.Concat_StrStr` "go move time " (`KismetStringLibrary.Conv_IntToString` (`self.MOVETIME`))))))

(fn `StringToCoord`
  (params (String :type String))
  (returns (fromX :type Integer) (fromY :type Integer) (toX :type Integer) (toY :type Integer))
  (locals (CharToInt :type "Map of String to Integer") (IntToInt :type "Map of String to Integer"))
  (bind _returnvalue (`KismetStringLibrary.GetCharacterArrayFromString` String))
  (bind _chartoint (`local.CharToInt`))
  (bind _inttoint (`local.IntToInt`))
  (return (`BlueprintMapLibrary.Map_Find` _chartoint (`|GetArrayItem` _returnvalue)) (`BlueprintMapLibrary.Map_Find` _inttoint (`|GetArrayItem` _returnvalue 1)) (`BlueprintMapLibrary.Map_Find` _chartoint (`|GetArrayItem` _returnvalue 2)) (`BlueprintMapLibrary.Map_Find` _inttoint (`|GetArrayItem` _returnvalue 3))))

(fn `UpdatePosition`
  (params (FENString :type String))
  (`self.SendCommand` (`KismetStringLibrary.Concat_StrStr` "position fen " FENString))
  (set `self.EngineState` "E_WAITING_FOR_COMMAND"))

(fn `UserConstructionScript`)