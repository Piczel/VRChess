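; BP_ChessBoard is the chess board actor, providing a function that spawns individual BP_ChessSquare actors for the board.
; SpawnChessSquare places each square by scaling its grid coordinate by PHYSICALSIZE and offsetting from the board's location, inheriting the board's rotation and scale.
; It branches on IsWhite to set the square's mesh material, though both branches currently assign M_ChessBoard.
; The event graph and construction script are empty, so nothing here calls the function.
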(event `self.ReceiveBeginPlay`)

(event `self.ReceiveEndPlay`
  (params (EndPlayReason :type "EEndPlayReason Enum" :default "Destroyed")))

(fn `SpawnChessSquare`
  (params (coord_x :type Integer) (coord_y :type Integer) (isWhite :type Boolean))
  (returns (ChessSquare :type "/Game/Chess/Blueprints/BP_ChessSquare Object Reference"))
  (bind _physical_size (`self.PHYSICAL_SIZE`))
  (bind _returnvalue (`|SpawnActorFromClass` "/Game/Chess/Blueprints/BP_ChessSquare.BP_ChessSquare_C" (`KismetMathLibrary.MakeTransform` (+ (`KismetMathLibrary.MakeVector` (* coord_x _physical_size) (* coord_y _physical_size)) (`self.K2_GetActorLocation`)) (`self.K2_GetActorRotation`) (`self.GetActorScale3D`)) "Undefined" "OverrideRootScale" null null))
  (if isWhite
    (bind _returnvalue_2 (`self.GetComponentByClass` _returnvalue "/Script/Engine.StaticMeshComponent"))
    (`PrimitiveComponent.SetMaterial` _returnvalue_2 0 "/Game/Chess/Materials/M_ChessBoard.M_ChessBoard")
    (else
      (`PrimitiveComponent.SetMaterial` _returnvalue_2 0 "/Game/Chess/Materials/M_ChessBoard.M_ChessBoard")))
  (return _returnvalue))

(fn `UserConstructionScript`)